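; Mantle component for ALS V4 characters; this graph picks which mantle asset to use for a climb.
; GetMantleAsset branches on mantle type: High Mantle and Falling Catch share the default 2m asset.
; Low Mantle also switches on overlay state, choosing default, left-hand, right-hand, two-hand or box 1m variants to suit the held item or pose.
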(fn GetMantleAsset
  (params (MantleType :type EALSMantleType%20Enum :default "HighMantle") (CurrentOverlayState :type EALSOverlayState%20Enum :default "Default"))
  (switch Utilities|FlowControl|Switch|SwitchonEALSMantleType MantleType
    (:HighMantle
      _)
    (:LowMantle
      (switch Utilities|FlowControl|Switch|SwitchonEALSOverlayState CurrentOverlayState
        (:Default
          _)
        (:Masculine
          _)
        (:Feminine
          _)
        (:Injured
          (return (Variables|Default|GetMantle_1m_LH)))
        (:HandsTied
          (return (Variables|Default|GetMantle_1m_2H)))
        (:Rifle
          (return (Variables|Default|GetMantle_1m_RH)))
        (:PistolOneHanded
          (return (Variables|Default|GetMantle_1m_RH)))
        (:PistolTwoHanded
          (return (Variables|Default|GetMantle_1m_RH)))
        (:Bow
          (return (Variables|Default|GetMantle_1m_LH)))
        (:Torch
          (return (Variables|Default|GetMantle_1m_LH)))
        (:Binoculars
          (return (Variables|Default|GetMantle_1m_RH)))
        (:Box
          (return (Variables|Default|GetMantle_1m_Box)))
        (:Barrel
          (return (Variables|Default|GetMantle_1m_LH))))
      (return (Variables|Default|GetMantle_1m_Default)))
    (:FallingCatch
      _))
  (return (Variables|Default|GetMantle_2m_Default)))