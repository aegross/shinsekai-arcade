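; Game instance for an arcade game that keeps player settings across the session and holds a shared game UI reference.
; On init it loads a BP_SaveSettings save, creating and saving defaults if the cast fails, and writes settings back on shutdown.
; ApplyVolume pushes doubled music, SFX and dialogue volumes into the master sound mix through class overrides.
; The player inventory getter and setter are empty stubs.
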(event EventInit
  ;[0.1986 0.06959 1] on game initialization, load settings, apply audio settings
  (CallFunction|LoadSettings)
  (CallFunction|ApplyVolume))

(event EventShutdown
  ;[0.1986 0.06959 1] on game shutdown, save settings
  (CallFunction|SaveSettings))

(fn LoadSettings
  (bind _settingsslot (Variables|Settings|GetSettingsSlot))
  ;[0.3372 0.06336 1] attempt to load settings-specific save
  (bind _returnvalue (SaveGame|LoadGamefromSlot _settingsslot))
  (bind _asbp_save_settings (Utilities|Casting|CastToBP_SaveSettings _returnvalue)
    (:then
      ;[0.3697 1 0.4709 1 12] if the cast is successful (settings were loaded), set settings according to file content
      (Variables|Settings|SetSettings _asbp_save_settings))
    (:CastFailed
      ;[1 0.2673 0.4836] if the cast is unsuccessful, save defaults to file
      (bind _returnvalue_2 (Game|ConstructObjectfromClass "/Game/Blueprints/StateManagement/BP_SaveSettings.BP_SaveSettings_C"))
      (bind _output_get (Variables|Settings|SetSettings _returnvalue_2))
      (bind _returnvalue_3 (SaveGame|SaveGametoSlot _output_get _settingsslot))
      (if (not _returnvalue_3)
        (Development|PrintString "Unable to save default settings.")))))

(fn SaveSettings
  (bind _returnvalue (SaveGame|SaveGametoSlot (Variables|Settings|GetSettings) (Variables|Settings|GetSettingsSlot)))
  (if (not _returnvalue)
    (Development|PrintString "Unable to save settings.")))

(fn ApplyVolume
  (bind _settings (Variables|Settings|GetSettings))
  (Utilities|FlowControl|Sequence
    (:then_0
      (Audio|SetSoundMixClassOverride "/Game/Audio/SCM_MasterMix.SCM_MasterMix" "/Game/Audio/SC_Music.SC_Music" (* (Variables|/Game/Blueprints/StateManagement/BP_SaveSettings.BP_SaveSettings_C|GetMusicVolume _settings) 2.0) 1.0 0.5 true))
    (:then_1
      (Audio|SetSoundMixClassOverride "/Game/Audio/SCM_MasterMix.SCM_MasterMix" "/Game/Audio/SC_SFX.SC_SFX" (* (Variables|/Game/Blueprints/StateManagement/BP_SaveSettings.BP_SaveSettings_C|GetSoundVolume _settings) 2.0) 1.0 0.05 true))
    (:then_2
      (Audio|SetSoundMixClassOverride "/Game/Audio/SCM_MasterMix.SCM_MasterMix" "/Game/Audio/SC_Dialogue.SC_Dialogue" (* (Variables|/Game/Blueprints/StateManagement/BP_SaveSettings.BP_SaveSettings_C|GetDialogueVolume _settings) 2.0) 1.0 0.05 true))))

(fn SetGameUI
  (params (GameUI :type WB%20Game%20UI%20Object%20Reference))
  (Variables|UI|SetGameUI GameUI))

(fn GetGameUI
  (return (Variables|UI|GetGameUI)))

(fn SetPlayerInventory
  (params (PlayerInventory :type AC%20Inventory%20System%20Object%20Reference)))

(fn GetPlayerInventory
  (return 0))