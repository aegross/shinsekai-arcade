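; BP_NPC_Base is a base Blueprint for NPCs that can show they are available to speak to and take part in conversations.
; The speak-state event toggles the name text and applies or clears an outline overlay material on the mesh and a temporary static mesh.
; The construction script fills the name text from NPCName.
; When a conversation closes, the NPC passes a closed message to its interaction instigator.
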(event EventConversationClosed
  (Class|BPIInteractableSpeak|ConversationClosed(Message) (Variables|Default|GetInteractInstigator)))

(event EventSetInteractableSpeakState
  (params (CanShowSpeak? :type Boolean))
  (bind _text_npcname (Variables|Default|GetText_NPCName))
  (bind _mesh (Variables|Character|GetMesh))
  (bind _tempmesh (Variables|Default|GetTempMesh))
  (if CanShowSpeak?
    ;[1 0 0.1641] show name text if interactable, show outline
    (Rendering|SetVisibility _text_npcname true false)
    (Rendering|Material|SetOverlayMaterial _mesh "/Game/Materials/BlueprintMaterials/M_Outline.M_Outline" :!class /Script/Engine.MeshComponent)
    ;[0 0.5547 1] this is temporary, only needed for static mesh
    (Rendering|Material|SetOverlayMaterial _tempmesh "/Game/Materials/BlueprintMaterials/M_Outline.M_Outline" :!class /Script/Engine.MeshComponent)
    (else
      (Rendering|SetVisibility _text_npcname false false)
      (Rendering|Material|SetOverlayMaterial _mesh 0 :!class /Script/Engine.MeshComponent)
      (Rendering|Material|SetOverlayMaterial _tempmesh 0 :!class /Script/Engine.MeshComponent))))

(fn ConstructionScript
  (Rendering|Components|TextRender|SetText (Variables|Default|GetText_NPCName) (Variables|Default|GetNPCName)))