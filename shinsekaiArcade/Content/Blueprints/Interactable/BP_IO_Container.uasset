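; BP_IO_Container is an interactable container that opens an inventory screen when interacted with.
; InteractObject calls the parent, then creates a container inventory widget bound to its inventory system component and itself, and stores the reference.
; The widget is added to the viewport and focused, with input switched to UI only and the mouse cursor shown.
; An unconnected leftover branch would instead show inventory through the game instance's game UI.
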(event EventInteractObject
  (params (Instigator :type Actor%20Object%20Reference))
  (bind _returnvalue (Game|GetPlayerController 0))
  (|CallParentFunction Instigator)
  ;[1 1 1] create the widget, add it to the viewport, focus it, and change the input mode to UI only
  (bind _returnvalue_2 (UserInterface|CreateWidget "/Game/UI/Inventory/WB_INV_ContainerInventory.WB_INV_ContainerInventory_C" 0 (Variables|Default|GetAC_InventorySystem_Container) self))
  (UserInterface|Viewport|AddtoViewport _returnvalue_2 0)
  (Variables|Default|SetInventoryWidget _returnvalue_2)
  (Input|SetInputModeUIOnly _returnvalue _returnvalue_2 "DoNotLock" false)
  (Variables|/Script/Engine.PlayerController|SetbShowMouseCursor _returnvalue true))

(fn ConstructionScript
  (|CallParentFunction))