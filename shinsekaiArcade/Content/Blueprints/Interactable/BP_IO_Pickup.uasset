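; Interactable pickup actor that moves its item into the interacting player's inventory.
; On interact it runs the parent logic, then passes the item ID and quantity from its item data component to the playable character's inventory component.
; On success it ends the interaction as destroyed and destroys itself, otherwise it prints an on-screen failure message.
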(event EventInteractObject
  (params (Instigator :type Actor%20Object%20Reference))
  (bind _ac_itemdatacomponent (Variables|Default|GetAC_ItemDataComponent))
  (|CallParentFunction Instigator)
  (bind _asbp_playable_character (Utilities|Casting|CastToBP_PlayableCharacter Instigator))
  (Utilities|IsValid (Variables|/Game/Blueprints/BP_PlayableCharacter.BP_PlayableCharacter_C|GetAC_InventorySystem _asbp_playable_character)
    (:Is%20Valid
      (bind _success (Default|AddtoInventory (Variables|/Game/Blueprints/BP_PlayableCharacter.BP_PlayableCharacter_C|GetAC_InventorySystem _asbp_playable_character) (.rowname (Variables|/Game/Inventory/AC_ItemDataComponent.AC_ItemDataComponent_C|GetItemID _ac_itemdatacomponent)) (Variables|/Game/Inventory/AC_ItemDataComponent.AC_ItemDataComponent_C|GetItemQuantity _ac_itemdatacomponent)))
      (if _success
        (Default|EndInteractionDestroyed (Variables|Default|GetAC_Interaction_Base))
        (Actor|DestroyActor)
        (else
          (Development|PrintString "Could not add item to inventory." true true "(R=1.000000,G=0.076447,B=0.144154,A=1.000000)"))))))

(fn ConstructionScript
  (|CallParentFunction))