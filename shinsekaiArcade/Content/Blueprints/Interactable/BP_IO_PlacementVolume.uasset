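; Interactable placement volume that holds one spawned, attached object and opens an interaction menu widget in UI-only input mode.
; While occupied, the hidden volume borrows the object's mesh, slightly enlarged, as its collision.
; Focus highlights the object through custom depth, or the empty volume through a material swap.
; Removal either sells the item using its data table value or returns it to player inventory, then restores the volume.
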(event EventSetInteractableState
  (params (CanShowInteract? :type Boolean))
  (bind _staticmesh (Variables|Default|GetStaticMesh))
  (if (Variables|Default|GetAllowInteraction?)
    (Utilities|FlowControl|Sequence
      (:then_0
        (bind _objectplaced (Variables|ObjectInfo|GetObjectPlaced)
          (:then
            (bind _asbp_object_base (Utilities|Casting|CastToBP_ObjectBase _objectplaced))
            (if CanShowInteract?
              (Rendering|SetRenderCustomDepth (Variables|/Game/Inventory/Items/BP_ObjectBase.BP_ObjectBase_C|GetStaticMesh _asbp_object_base) true)
              (else
                (Rendering|SetRenderCustomDepth (Variables|/Game/Inventory/Items/BP_ObjectBase.BP_ObjectBase_C|GetStaticMesh _asbp_object_base) false))))
          (:else)))
      (:then_1
        (if (not (Variables|ObjectInfo|GetContainsObject?))
          (if CanShowInteract?
            (Rendering|Material|SetMaterial _staticmesh 0 "/Game/Materials/BlueprintMaterials/M_SemiTransparent_PV_Interact.M_SemiTransparent_PV_Interact")
            (else
              (Rendering|Material|SetMaterial _staticmesh 0 "/Game/Materials/BlueprintMaterials/M_SemiTransparent_PV.M_SemiTransparent_PV"))))))))

(event EventInteractObject
  (params (Instigator :type Actor%20Object%20Reference))
  (bind _returnvalue (Game|GetPlayerController 0))
  (|CallParentFunction Instigator)
  (if (Variables|Default|GetAllowInteraction?)
    ;[1 1 1] create the widget, add it to the viewport, focus it, and change the input mode to UI only
    (bind _returnvalue_2 (UserInterface|CreateWidget "/Game/UI/ObjectInteraction/WB_InteractionMenu.WB_InteractionMenu_C" 0 self "NewEnumerator0" (Variables|ObjectInfo|GetObjectItemID)))
    (UserInterface|Viewport|AddtoViewport _returnvalue_2 0)
    (bind _output_get (Variables|Default|SetInteractionMenuWidget _returnvalue_2))
    (Input|SetInputModeUIOnly _returnvalue _output_get "DoNotLock" false)
    (Variables|/Script/Engine.PlayerController|SetbShowMouseCursor _returnvalue true)
    (else
      (Default|EndInteraction (Variables|Default|GetAC_Interaction_Base) false))))

(event EventBeginPlay
  (bind _staticmesh (Variables|Default|GetStaticMesh))
  (bind _staticmesh_2 (Variables|Default|GetStaticMesh))
  (bind _relativelocation (Variables|/Script/Engine.SceneComponent|GetRelativeLocation _staticmesh))
  (Variables|VolumeInfo|SetPlacementLocation _relativelocation)
  (Variables|VolumeInfo|SetInteractionLocation (+ _relativelocation ""))
  ;[0 0.5641 1] placement volumes don't change size during their lifespan
  (Variables|Mesh|SetOriginalStaticMesh (Variables|/Script/Engine.StaticMeshComponent|GetStaticMesh _staticmesh_2))
  (Variables|Mesh|SetOriginalRelativeScale (Variables|/Script/Engine.SceneComponent|GetRelativeScale3D _staticmesh_2)))

(fn ConstructionScript
  (|CallParentFunction))

(fn GetPlacementRestrictions
  (return (Variables|ObjectInfo|GetAllowedObjectTypes) (Variables|ObjectInfo|GetAllowedObjectSizes)))

(fn GetObjectClass
  (bind _objectplaced (Variables|ObjectInfo|GetObjectPlaced))
  (bind _returnvalue (Utilities|GetClass _objectplaced))
  ;[0 0 0] wrote this and then realized it was probably completely unnecessary :D
  (if (Variables|ObjectInfo|GetContainsObject?)
    (Development|PrintString (Utilities|GetClassDisplayName _returnvalue))
    (return _returnvalue)
    (else
      (return 0))))

(fn SetObject
  (params (NewObjectActorClass :type Actor%20Class%20Reference) (ItemID :type Name))
  (bind _staticmesh (Variables|Default|GetStaticMesh))
  ;[0 0.2969 1] If the class is the same, either don't do anything or reset object attributes
  (if (!= NewObjectActorClass (Utilities|GetClass (Variables|ObjectInfo|GetObjectPlaced)))
    (Variables|ObjectInfo|SetObjectItemID ItemID)
    (bind _returnvalue (Game|SpawnActorfromClass NewObjectActorClass (Math|Transform|MakeTransform (Variables|VolumeInfo|GetPlacementLocation)) "AdjustIfPossibleButAlwaysSpawn" "MultiplyWithRoot" 0 0))
    (Transformation|AttachActorToActor _returnvalue self "None" "KeepRelative" "KeepRelative" "KeepRelative" true)
    (Rendering|SetVisibility (Variables|Default|GetStaticMesh) false false)
    (Variables|ObjectInfo|SetObjectPlaced _returnvalue)
    (Variables|ObjectInfo|SetContainsObject? true)
    ;[0 0.5069 1] collision nonsense since it's a child and not a component... whatever
    (bind _asbp_object_base (Utilities|Casting|CastToBP_ObjectBase _returnvalue))
    (bind _output_get (Variables|Mesh|SetPlacedStaticMesh (Variables|/Script/Engine.StaticMeshComponent|GetStaticMesh (Variables|/Game/Inventory/Items/BP_ObjectBase.BP_ObjectBase_C|GetStaticMesh _asbp_object_base))))
    (Components|StaticMesh|SetStaticMesh _staticmesh _output_get)
    (Transformation|SetRelativeScale3D _staticmesh (* (Variables|/Script/Engine.SceneComponent|GetRelativeScale3D (Variables|/Game/Inventory/Items/BP_ObjectBase.BP_ObjectBase_C|GetDefaultSceneRoot _asbp_object_base)) "1.050000,1.050000,1.050000"))))

(fn RemoveObject
  (params (RemoveAndSell? :type Boolean))
  (bind _staticmesh (Variables|Default|GetStaticMesh))
  (Utilities|FlowControl|Sequence
    (:then_0
      (if RemoveAndSell?
        ;[1 1 1] sell the object
        (bind _asbp_third_person_gamemode_als (Utilities|Casting|CastToBP_ThirdPersonGamemode_ALS (Game|GetGameMode)))
        (bind _returnvalue (Utilities|GetDataTableRow "/Game/Inventory/DT_ItemData.DT_ItemData" (Variables|ObjectInfo|GetObjectItemID))
          (:then
            (Default|AlterMoney _asbp_third_person_gamemode_als (.ValueYen (Utilities|Struct|BreakSTR_InventoryItem _returnvalue))))
          (:RowNotFound
            (Default|AlterMoney _asbp_third_person_gamemode_als)))
        (else
          ;[0.4241 1 0] try to add it to the player's inventory
          (bind _asbp_arcade_player_controller_als (Utilities|Casting|CastToBP_ArcadePlayerController_ALS (Game|GetPlayerController 0)))
          (bind _success (Default|AddtoInventory (Variables|/Game/Blueprints/Input/PlayerControllers/BP_ArcadePlayerController_ALS.BP_ArcadePlayerController_ALS_C|GetAC_Player_InventorySystem _asbp_arcade_player_controller_als) (Variables|ObjectInfo|GetObjectItemID) 1))
          (if (not _success)
            (Development|PrintText "item could not be added to inventory. it will not be removed." true true "(R=1.000000,G=0.000000,B=0.286160,A=1.000000)")
            (return false) ; short-circuit the function
          ))))
    (:then_1
      ;[1 0 0.2812] remove all actors and references, make volume visible again
      (Actor|DestroyActor (Variables|ObjectInfo|GetObjectPlaced))
      (Variables|ObjectInfo|SetObjectPlaced 0)
      (Variables|ObjectInfo|SetObjectItemID "None")
      (Variables|ObjectInfo|SetContainsObject? false)
      (Variables|Mesh|SetPlacedStaticMesh 0)
      (Components|StaticMesh|SetStaticMesh _staticmesh (Variables|Mesh|GetOriginalStaticMesh))
      (Transformation|SetRelativeScale3D _staticmesh (Variables|Mesh|GetOriginalRelativeScale))
      (Rendering|SetVisibility _staticmesh true false)
      (return true))))

(fn SetAllowInteraction
  (params (AllowInteraction? :type Boolean))
  (bind _staticmesh (Variables|Default|GetStaticMesh))
  (if AllowInteraction?
    (Variables|Default|SetAllowInteraction? true)
    ;[0.06541 0 1] allow/disallow the trace to "pick up" the object
    (Collision|SetCollisionResponsetoChannel _staticmesh "ECC_Visibility" "ECR_Block")
    (if (Variables|ObjectInfo|GetContainsObject?)
      (Rendering|SetVisibility _staticmesh false false)
      (else
        (Rendering|SetVisibility _staticmesh true false)))
    (else
      (Variables|Default|SetAllowInteraction? false)
      (Collision|SetCollisionResponsetoChannel _staticmesh "ECC_Visibility" "ECR_Ignore")
      (Rendering|SetVisibility _staticmesh false false))))