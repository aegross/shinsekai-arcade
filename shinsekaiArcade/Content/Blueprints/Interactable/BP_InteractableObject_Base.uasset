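; Base Blueprint for interactable objects that can be highlighted and report their item details when interacted with.
; Toggles an outline overlay material on the static mesh to show interactability.
; On interaction it stores the instigator, then prints the item name and description from the data table row referenced by its item data component.
; When interaction closes, it notifies that instigator whether the object was destroyed.
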(event EventSetInteractableState
  (params (CanShowInteract? :type Boolean))
  (bind _staticmesh (Variables|Default|GetStaticMesh))
  (if CanShowInteract?
    ;[1 0.7031 0] this is for static meshes only
    (Rendering|Material|SetOverlayMaterial _staticmesh "/Game/Materials/BlueprintMaterials/M_Outline.M_Outline" :!class /Script/Engine.MeshComponent)
    (else
      (Rendering|Material|SetOverlayMaterial _staticmesh 0 :!class /Script/Engine.MeshComponent))))

(event EventInteractObject
  (params (Instigator :type Actor%20Object%20Reference))
  (Variables|Components|SetInteractInstigator Instigator)
  (Testing|PrintObjectInfo))

(event EventInteractionClosed
  (params (ObjectDestroyed :type Boolean))
  (Class|BPIInteractableInteract|InteractionClosed(Message) (Variables|Components|GetInteractInstigator) ObjectDestroyed))

(fn ConstructionScript)

(fn GetObjectInfo
  (bind _ac_itemdatacomponent (Variables|Default|GetAC_ItemDataComponent))
  (bind _itemid (Variables|/Game/Inventory/AC_ItemDataComponent.AC_ItemDataComponent_C|GetItemID _ac_itemdatacomponent))
  (bind _returnvalue (Utilities|GetDataTableRow (.datatable _itemid) (.rowname _itemid))
    (:then
      (return _returnvalue))))

(fn PrintObjectInfo
  (bind _inventoryiteminfo (CallFunction|GetObjectInfo))
  (Development|PrintText (Utilities|Text|FormatText "Item Name: {itemName} 
Item Description: {itemDesc}" (.itemname _inventoryiteminfo) (.itemdescription _inventoryiteminfo)) true false "(R=0.142777,G=0.085059,B=1.000000,A=1.000000)"))