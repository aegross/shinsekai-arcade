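; BP_PlacementVolume is an interactable slot that holds one placed object through a ChildActor component.
; Interacting creates and stores a WB_InteractionMenu widget, then switches to UI-only input with a visible cursor.
; SetObject swaps the child actor class if it differs, records the placed actor and hides the static mesh.
; RemoveObject clears the slot and shows the mesh again, ignoring its sell flag; PlaceObjectActor is an empty stub.
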(event EventInteractObject
  (params (Instigator :type Actor%20Object%20Reference))
  (bind _returnvalue (Game|GetPlayerController 0))
  ;[1 1 1] create the widget, add it to the viewport, focus it, and change the input mode to UI only
  (|CallParentFunction Instigator)
  (bind _returnvalue_2 (UserInterface|CreateWidget "/Game/UI/ObjectInteraction/WB_InteractionMenu.WB_InteractionMenu_C" 0 self))
  (UserInterface|Viewport|AddtoViewport _returnvalue_2 0)
  (Variables|Default|SetInteractionMenuWidget _returnvalue_2)
  (Input|SetInputModeUIOnly _returnvalue 0 "DoNotLock" false)
  (Variables|/Script/Engine.PlayerController|SetbShowMouseCursor _returnvalue true))

(event EventBeginPlay
  (bind _objectactor (Variables|Default|GetObjectActor))
  (bind _returnvalue (Transformation|GetWorldLocation _objectactor))
  (Variables|VolumeInfo|SetPlacementLocation _returnvalue)
  (Variables|VolumeInfo|SetInteractionLocation (+ _returnvalue "")))

(fn ConstructionScript
  (|CallParentFunction))

(fn SetObject
  (params (NewObjectActorClass :type Actor%20Class%20Reference))
  (bind _objectactor (Variables|Default|GetObjectActor))
  ;[0 0.2969 1] If the class is the same, either don't do anything or reset object attributes
  (bind _output_get (LocalVariables|SetLOCAL_PreviousActorClass (Variables|/Script/Engine.ChildActorComponent|GetChildActorClass _objectactor)))
  (if (!= _output_get NewObjectActorClass)
    (ChildActorComponent|SetChildActorClass _objectactor NewObjectActorClass)
    (Rendering|SetVisibility (Variables|Default|GetStaticMesh) false false)
    (Variables|ObjectInfo|SetObjectPlaced (Variables|/Script/Engine.ChildActorComponent|GetChildActor (Variables|Default|GetObjectActor)))
    (Variables|ObjectInfo|SetContainsObject? true)))

(fn PlaceObjectActor)

(fn RemoveObject
  (params (RemoveAndSell? :type Boolean))
  (ChildActorComponent|SetChildActorClass (Variables|Default|GetObjectActor) "/Script/Engine.Actor")
  (Variables|ObjectInfo|SetObjectPlaced 0)
  (Variables|ObjectInfo|SetContainsObject? false)
  (Rendering|SetVisibility (Variables|Default|GetStaticMesh) true false))