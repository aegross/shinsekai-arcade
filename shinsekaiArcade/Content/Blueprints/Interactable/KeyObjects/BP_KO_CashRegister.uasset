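; BP_KO_CashRegister is an interactable key object for a cash register that opens a register menu when used.
; On interaction it runs the parent logic, creates WB_RegisterMenu with itself as the register actor, adds it to the viewport, and switches player 0 to UI-only input with a visible cursor.
; Closing the interaction and construction only call the parent implementations, with no input restore in this Blueprint.
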(event EventInteractObject
  (params (Instigator :type Actor%20Object%20Reference))
  (bind _returnvalue (Game|GetPlayerController 0))
  (|CallParentFunction Instigator)
  (bind _returnvalue_2 (UserInterface|CreateWidget "/Game/UI/ObjectInteraction/WB_RegisterMenu.WB_RegisterMenu_C" 0 self))
  (UserInterface|Viewport|AddtoViewport _returnvalue_2 0)
  (Input|SetInputModeUIOnly _returnvalue _returnvalue_2 "DoNotLock" false)
  (Variables|/Script/Engine.PlayerController|SetbShowMouseCursor _returnvalue true))

(event EventInteractionClosed
  (params (ObjectDestroyed :type Boolean))
  (|CallParentFunction ObjectDestroyed))

(fn ConstructionScript
  (|CallParentFunction))