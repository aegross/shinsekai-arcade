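; BP_KO_Catalog is an interactable key object that opens the catalog menu when a player interacts with it.
; It creates a WB_CatalogMenu linked to itself, flagged unusable when the ALS game mode's phase differs from one specific value.
; A failed game mode cast opens the default menu.
; Input then switches to UI-only with a visible cursor, with focus always targeting the default-branch widget variable.
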(event EventInteractObject
  (params (Instigator :type Actor%20Object%20Reference))
  (bind _returnvalue (Game|GetPlayerController 0))
  (bind _self self)
  (|CallParentFunction Instigator)
  (bind _asbp_third_person_gamemode_als (Utilities|Casting|CastToBP_ThirdPersonGamemode_ALS (Game|GetGameMode))
    (:then
      (if (Utilities|Enum|Equal(Enum) (Variables|/Game/Blueprints/Gamemodes/BP_ThirdPersonGamemode_ALS.BP_ThirdPersonGamemode_ALS_C|GetGamePhase _asbp_third_person_gamemode_als) "NewEnumerator3")
        (bind _returnvalue_2 (UserInterface|CreateWidget "/Game/UI/ObjectInteraction/WB_CatalogMenu.WB_CatalogMenu_C" 0 _self :!label _label))
        (UserInterface|Viewport|AddtoViewport _returnvalue_2 0)
        (else
          (bind _returnvalue_3 (UserInterface|CreateWidget "/Game/UI/ObjectInteraction/WB_CatalogMenu.WB_CatalogMenu_C" 0 _self false))
          (UserInterface|Viewport|AddtoViewport _returnvalue_3 0))))
    (:CastFailed
      (goto _label)))
  (Input|SetInputModeUIOnly _returnvalue _returnvalue_2 "DoNotLock" false)
  (Variables|/Script/Engine.PlayerController|SetbShowMouseCursor _returnvalue true))

(event EventInteractionClosed
  (params (ObjectDestroyed :type Boolean))
  (|CallParentFunction ObjectDestroyed))

(fn ConstructionScript
  (|CallParentFunction))