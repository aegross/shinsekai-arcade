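; BP_KO_DeskHinge is an interactable key object for a desk hinge that swings open and shut.
; On interaction it snaps the root component's relative rotation between zero and 90 degrees with no animation, toggling IsOpen.
; Returning to the closed rotation also sets its interactable state to false.
; Each interaction runs the parent logic first and ends by calling InteractionClosed without flagging the object as destroyed.
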(event EventInteractObject
  (params (Instigator :type Actor%20Object%20Reference))
  (bind _defaultsceneroot (Variables|Default|GetDefaultSceneRoot))
  (|CallParentFunction Instigator)
  (if (Variables|Default|GetIsOpen?)
    (Transformation|SetRelativeRotation _defaultsceneroot "0, 0, 0" false false)
    (CallFunction|SetInteractableState false)
    (else
      (Transformation|SetRelativeRotation _defaultsceneroot "90.000000,0.000000,0.000000" false false)))
  (Variables|Default|SetIsOpen? (not (Variables|Default|GetIsOpen?)))
  (Default|InteractionClosed self false))

(event EventInteractionClosed
  (params (ObjectDestroyed :type Boolean))
  (|CallParentFunction ObjectDestroyed))

(fn ConstructionScript
  (|CallParentFunction))