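; BP_KO_OpenCloseSign is an interactable open/close sign that lets the player advance the arcade's game phase.
; Interacting opens a WB_ConfirmationDialog with Yes and No buttons bound to its events.
; Yes calls UpdateGamePhase on ArcadeLevelManager, closes the dialog, restores game input, and snaps the sign's rotation to match the returned phase.
; No only sends a manual interaction-closed message to the instigator.
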(event Custom|OnInteractYes
  (bind _returnvalue (Game|GetPlayerController 0))
  (bind _result_game_phase (Default|UpdateGamePhase (Variables|Default|GetArcadeLevelManager)))
  (Utilities|FlowControl|Sequence
    (:then_0
      ;[0 0.3521 1] mostly widget stuff
      (Widget|RemovefromParent (Variables|Default|GetConfirmationWidget))
      (Input|SetInputModeGameOnly _returnvalue false)
      (Variables|/Script/Engine.PlayerController|SetbShowMouseCursor _returnvalue false)
      (Class|BPIInteractableInteract|InteractionClosed(Message) (Variables|Default|GetInteractInstigator) false))
    (:then_1
      (if (Utilities|Enum|Equal(Enum) _result_game_phase "NewEnumerator2")
        ;[0 0.6733 1] TODO change to animated sequence
        (Transformation|SetActorRelativeRotation "0, 0, 0")
        (else
          (Transformation|SetActorRelativeRotation "0.000000,-180.000000,0.000000"))))))

(event Custom|OnInteractNo
  ;[1 0 0] the notify has to be manual for some reason
  (Class|BPIInteractableInteract|InteractionClosed(Message) (Variables|Default|GetInteractInstigator) false))

(event EventInteractionClosed
  (params (ObjectDestroyed :type Boolean))
  (|CallParentFunction ObjectDestroyed))

(event EventInteractObject
  (params (Instigator :type Actor%20Object%20Reference))
  (|CallParentFunction Instigator)
  (bind _returnvalue (UserInterface|CreateWidget "/Game/UI/WB_ConfirmationDialog.WB_ConfirmationDialog_C" 0 "Are you sure that you want to advance to the next game phase?"))
  (bind _output_get (Variables|Default|SetConfirmationWidget _returnvalue))
  (UserInterface|Viewport|AddtoViewport _output_get 0)
  (EventDispatchers|BindEventtoOnClicked (Variables|/Game/UI/WB_ConfirmationDialog.WB_ConfirmationDialog_C|Getbutton_yes (Variables|Default|GetConfirmationWidget)) (delegate Custom|OnInteractYes))
  (EventDispatchers|BindEventtoOnClicked (Variables|/Game/UI/WB_ConfirmationDialog.WB_ConfirmationDialog_C|Getbutton_no (Variables|Default|GetConfirmationWidget)) (delegate Custom|OnInteractNo)))

(fn ConstructionScript
  (|CallParentFunction))