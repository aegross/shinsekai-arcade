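; BP_KO_DeskHinge is an interactable key object, named as a desk hinge, that toggles between an open and a closed rotation.
; On InteractObject it runs the parent logic, then snaps DefaultSceneRoot's relative rotation to OpenRotation or ClosedRotation and flips IsOpen, with no animation.
; Interaction closing, interactable state and construction pass straight through to the parent Blueprint.
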(event EventInteractionClosed
  (params (ObjectDestroyed :type Boolean))
  (|CallParentFunction ObjectDestroyed))

(event EventSetInteractableState
  (params (CanShowInteract? :type Boolean))
  (|CallParentFunction CanShowInteract?))

(event EventInteractObject
  (params (Instigator :type Actor%20Object%20Reference))
  (bind _defaultsceneroot (Variables|Default|GetDefaultSceneRoot))
  (|CallParentFunction Instigator)
  (if (Variables|Default|GetIsOpen?)
    (Transformation|SetRelativeRotation _defaultsceneroot (Variables|Default|GetClosedRotation) false false)
    (else
      (Transformation|SetRelativeRotation _defaultsceneroot (Variables|Default|GetOpenRotation) false false)))
  (Variables|Default|SetIsOpen? (not (Variables|Default|GetIsOpen?))))

(fn ConstructionScript
  (|CallParentFunction))