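; Test NPC dialogue component that scripts a branching introduction conversation with selectable player responses.
; The Dialogue override switches on ActiveBranch, chaining AddDialogue calls that advance on Passthrough and fork on the chosen option.
; The IRS answer permanently switches to branch 1, which picks a random nervous line, while other answers reset to the introduction.
; A helper builds each line struct with the speaker's name and color.
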(fn Dialogue
  (bind _array (Utilities|Array|MakeArray "Continue"))
  ;[0 0 0] beginning of dialogue sequence
  (|CallParentFunction)
  (switch int (Variables|Default|GetActiveBranch)
    (:0
      (bind _dialogueline (CallFunction|CreateGenericDialogueLineTest "Hi there! I'm TestNPC. Who are you?" (Utilities|Array|MakeArray "A member of the IRS." "A student from WPI." "A student from Ritsumeikan.")))
      (bind (_dialoguestate _optionindex) (CallFunction|AddDialogue _dialogueline))
      (switch Utilities|FlowControl|Switch|SwitchonENUM_DialogueState _dialoguestate
        (:NewEnumerator0
          (switch int _optionindex
            (:0
              (bind _dialogueline_2 (CallFunction|CreateGenericDialogueLineTest "I've done my taxes, I swear!" _array))
              (bind _dialoguestate_2 (CallFunction|AddDialogue _dialogueline_2))
              (switch Utilities|FlowControl|Switch|SwitchonENUM_DialogueState _dialoguestate_2
                (:NewEnumerator0
                  (CallFunction|SetActiveBranch 1)
                  (CallFunction|ClearDialogueProgress)
                  (CallFunction|CloseConversation))))
            (:1
              (bind _dialogueline_3 (CallFunction|CreateGenericDialogueLineTest "Cool! Nice to meet you!" _array))
              (bind _dialoguestate_3 (CallFunction|AddDialogue _dialogueline_3))
              (switch Utilities|FlowControl|Switch|SwitchonENUM_DialogueState _dialoguestate_3
                (:NewEnumerator0
                  ;[1 0 0.1172] reset to the beginning
                  (CallFunction|ClearDialogueProgress :!label _label)
                  (CallFunction|CloseConversation))))
            (:2
              (bind _dialogueline_4 (CallFunction|CreateGenericDialogueLineTest "Wow, neat! It's nice to meet you!" _array))
              (bind _dialoguestate_4 (CallFunction|AddDialogue _dialogueline_4))
              (switch Utilities|FlowControl|Switch|SwitchonENUM_DialogueState _dialoguestate_4
                (:NewEnumerator0
                  (goto _label))))))))
    (:1
      (bind _dialogueline_5 (CallFunction|CreateGenericDialogueLineTest (Utilities|Select :Index (Math|Random|RandomIntegerinRange 0 1) :Option%200 "Uhh... please don't tell me you need something." :Option%201 "You can see my tax returns if you need them!") (Utilities|Array|MakeArray "[Leave]")))
      (bind _dialoguestate_5 (CallFunction|AddDialogue _dialogueline_5))
      (switch Utilities|FlowControl|Switch|SwitchonENUM_DialogueState _dialoguestate_5
        (:NewEnumerator0
          (CallFunction|ClearDialogueProgress)
          (CallFunction|CloseConversation))))))

(fn CreateGenericDialogueLineTest
  (params (DialogueText :type Text) (ResponseOptions :type Array%20of%20Texts))
  (return (Utilities|String|Len (Utilities|String|ToString(Text) DialogueText)) (Utilities|Struct|MakeSTR_DialogueLine "NewEnumerator0" "NewEnumerator0" "Regular" (Variables|Default|GetSpeakerText) DialogueText ResponseOptions (Variables|Default|GetSpeakerColor))))