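; Inventory component that stores items in a fixed-size array of ID and quantity slots.
; Adding fills matching stacks one item at a time before claiming empty slots, with stack limits and item classes read from DT_ItemData.
; Transfers between inventories merge or swap slots, while removal can spawn the item ahead of the player and using spawns its effect actor.
; Removals and transfers fire OnInventoryUpdated; adding does not.
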(event Custom|UpdateInventory
  (Default|CallOnInventoryUpdated))

(event EventBeginPlay
  (Utilities|Array|Resize (Variables|Default|GetInventoryContent) (Variables|Default|GetInventorySize)))

(fn AddtoInventory
  (params (ItemID :type Name) (Quantity :type Integer))
  (LocalVariables|SetLocal_QuantityRemaining Quantity)
  (while (and (> (LocalVariables|GetLocal_QuantityRemaining) 0) (not (LocalVariables|GetLocal_HasFailed)))
    ;[0 0.0278 1] if a slot is found, add the item to that slot (if it's not full). otherwise, make a new slot
    (bind (_slotindex _foundslot_) (Helper|FindSlot ItemID))
    (if _foundslot_
      (Helper|AddtoStack _slotindex 1)
      (Math|Integer|DecrementInt (LocalVariables|GetLocal_QuantityRemaining))
      (elif (.HasEmptySlot (Helper|EmptySlotsAvailable?))
        (bind _success (Helper|CreateNewStack ItemID 1))
        (if _success
          (Math|Integer|DecrementInt (LocalVariables|GetLocal_QuantityRemaining))
          (else
            (LocalVariables|SetLocal_HasFailed true)))
        (else
          (LocalVariables|SetLocal_HasFailed true)))))
  (return (not (LocalVariables|GetLocal_HasFailed)) (LocalVariables|GetLocal_QuantityRemaining)))

(fn RemovefromInventory
  (params (Index :type Integer) (RemoveAll? :type Boolean) (IsConsumed? :type Boolean))
  (bind _inventorycontent (Variables|Default|GetInventoryContent))
  (bind _inventorycontent_2 (Variables|Default|GetInventoryContent))
  (bind _output (Utilities|Array|Get(acopy) _inventorycontent Index))
  (bind _output_2 (Utilities|Array|Get(acopy) _inventorycontent_2 Index))
  (LocalVariables|SetLOCAL_ItemID (.itemid _output))
  (LocalVariables|SetLOCAL_ItemQuantity (.quantity _output))
  (Utilities|FlowControl|Sequence
    (:then_0
      (if (or RemoveAll? (== (LocalVariables|GetLOCAL_ItemQuantity) 1))
        ;[1 0 0.0763] delete all of the items in that slot
        (Utilities|Array|SetArrayElem (Variables|Default|GetInventoryContent) Index (Utilities|Struct|MakeSTR_InventorySlot "None" 0))
        (else
          (Utilities|Struct|SetmembersinSTR_InventorySlot _output_2 (- (.Quantity (Utilities|Struct|BreakSTR_InventorySlot _output_2)) 1))))
      (if (not IsConsumed?)
        ;[1 0 0.5386] place object in world
        (CallFunction|PlaceItem(Helper) (LocalVariables|GetLOCAL_ItemID))))
    (:then_1
      (CallFunction|UpdateInventory))))

(fn FindSlot
  (params (ItemID :type Name))
  (for (_array_element _array_index) (Variables|Default|GetInventoryContent)
    (if (== (.ItemID (Utilities|Struct|BreakSTR_InventorySlot _array_element)) ItemID)
      (if (< (.Quantity (Utilities|Struct|BreakSTR_InventorySlot _array_element)) (Helper|GetMaxStackSize ItemID))
        (return _array_index true) ; a slot was found, return true along with the array index
      )))
  (return -1 false) ; no slot was found, return false along with -1
)

(fn AddtoStack
  (params (InventoryIndex :type Integer) (Quantity :type Integer))
  (bind _inventorycontent (Variables|Default|GetInventoryContent))
  (bind _output (Utilities|Array|Get(acopy) _inventorycontent InventoryIndex))
  (Utilities|Array|SetArrayElem (Variables|Default|GetInventoryContent) InventoryIndex (Utilities|Struct|MakeSTR_InventorySlot (.itemid _output) (+ (.quantity _output) Quantity))))

(fn GetMaxStackSize
  (params (ItemID :type Name))
  (bind _returnvalue (Utilities|GetDataTableRow "/Game/Inventory/DT_ItemData.DT_ItemData" ItemID)
    (:then
      (return (.StackSize (Utilities|Struct|BreakSTR_InventoryItem _returnvalue))))
    (:RowNotFound
      ;[0 0.133 1] item doesn't exist in data table
      (return -1))))

(fn GetItemData
  (params (ItemID :type Name))
  (bind _returnvalue (Utilities|GetDataTableRow "/Game/Inventory/DT_ItemData.DT_ItemData" ItemID)
    (:then
      (return _returnvalue))))

(fn EmptySlotsAvailable?
  (for (_array_element _array_index) (Variables|Default|GetInventoryContent)
    (if (== (.Quantity (Utilities|Struct|BreakSTR_InventorySlot _array_element)) 0)
      (return true _array_index)))
  (return false -1))

(fn CreateNewStack
  (params (ItemID :type Name) (Quantity :type Integer))
  (bind (_hasemptyslot _firstemptyindex) (Helper|EmptySlotsAvailable?))
  (if _hasemptyslot
    (Utilities|Array|SetArrayElem (Variables|Default|GetInventoryContent) _firstemptyindex (Utilities|Struct|MakeSTR_InventorySlot ItemID Quantity))
    (return true 0)
    (else
      (return false 0))))

(fn GetPlacementLocation
  (bind _returnvalue (Game|GetPlayerCharacter 0))
  ;[1 0.8837 0] This WILL be more complicated at some point, and will likely use other functions created later (having to do with "slots" that objects can be placed in)
  (return (+ (Transformation|GetActorLocation _returnvalue) (* (Transformation|GetActorForwardVector _returnvalue) (Variables|Default|GetPlacementDistance)))))

(fn DEVPrintContents
  (for (_array_element _array_index) (Variables|Default|GetInventoryContent)
    (Development|PrintString (Utilities|String|Append (Utilities|String|ToString(Integer) _array_index) ": " (Utilities|String|ToString(Name) (.ItemID (Utilities|Struct|BreakSTR_InventorySlot _array_element))) " = " (Utilities|String|ToString(Integer) (.Quantity (Utilities|Struct|BreakSTR_InventorySlot _array_element)))) true true "(R=0.111317,G=0.497692,B=1.000000,A=1.000000)")))

(fn TransferSlots
  (params (SourceIndex :type Integer) (Source%20Inventory :type AC%20Inventory%20System%20Object%20Reference) (DestinationIndex :type Integer))
  (bind _inventorycontent (Variables|Default|GetInventoryContent))
  (bind _output (Utilities|Array|Get(acopy) _inventorycontent DestinationIndex))
  (bind _stacksize (Helper|GetMaxStackSize (.itemid _output)))
  (LocalVariables|SetLOCAL_SourceInventoryContent (Utilities|Array|Get(acopy) (Variables|AC_InventorySystem_C|GetInventoryContent Source%20Inventory) SourceIndex))
  (if (not (< DestinationIndex 0))
    (if (== (.ItemID (Utilities|Struct|BreakSTR_InventorySlot (LocalVariables|GetLOCAL_SourceInventoryContent))) (.ItemID (Utilities|Struct|BreakSTR_InventorySlot (Utilities|Array|Get(acopy) (Variables|Default|GetInventoryContent) DestinationIndex))))
      (Utilities|Array|SetArrayElem (Variables|AC_InventorySystem_C|GetInventoryContent Source%20Inventory) SourceIndex (Utilities|Struct|MakeSTR_InventorySlot (select (> (Math|Integer|Clamp(Integer) (- (+ (.quantity _output) (.quantity (LocalVariables|GetLOCAL_SourceInventoryContent))) _stacksize) 0 _stacksize) 0) (.itemid (LocalVariables|GetLOCAL_SourceInventoryContent)) "None") (Math|Integer|Clamp(Integer) (- (+ (.quantity _output) (.quantity (LocalVariables|GetLOCAL_SourceInventoryContent))) _stacksize) 0 _stacksize))) ; set slot with remainder (if necessary)
      (Utilities|Array|SetArrayElem (Variables|Default|GetInventoryContent) DestinationIndex (Utilities|Struct|MakeSTR_InventorySlot (.itemid (LocalVariables|GetLOCAL_SourceInventoryContent)) (Math|Integer|Clamp(Integer) (+ (.quantity _output) (.quantity (LocalVariables|GetLOCAL_SourceInventoryContent))) 0 (Helper|GetMaxStackSize (.itemid (LocalVariables|GetLOCAL_SourceInventoryContent)))))) ; set slot with amount
      ;[1 1 1] update (refresh) inventories
      (CallFunction|UpdateInventory Source%20Inventory)
      (CallFunction|UpdateInventory self)
      (else
        (Utilities|Array|SetArrayElem (Variables|AC_InventorySystem_C|GetInventoryContent Source%20Inventory) SourceIndex (Utilities|Array|Get(acopy) (Variables|Default|GetInventoryContent) DestinationIndex)) ; when the item types don't match, swap the contents of the two slots
        (Utilities|Array|SetArrayElem (Variables|Default|GetInventoryContent) DestinationIndex (LocalVariables|GetLOCAL_SourceInventoryContent))
        (CallFunction|UpdateInventory)
        (CallFunction|UpdateInventory Source%20Inventory)))))

(fn UseItem
  (params (Index :type Integer))
  (bind _inventorycontent (Variables|Default|GetInventoryContent))
  (bind _output (Utilities|Array|Get(acopy) _inventorycontent Index))
  (LocalVariables|SetLOCAL_ItemID (.itemid _output))
  (LocalVariables|SetLOCAL_ItemQuantity (.quantity _output))
  (Utilities|FlowControl|Sequence
    (:then_0
      (CallFunction|RemovefromInventory Index false true)
      ;[0.2104 0 1] "use item" effect
      (Game|SpawnActorfromClass (.ItemEffect (Utilities|Struct|BreakSTR_InventoryItem (Helper|GetItemData (LocalVariables|GetLOCAL_ItemID)))) (Math|Transform|MakeTransform "0, 0, 0") "Undefined" "MultiplyWithRoot" 0 0))
    (:then_1
      (CallFunction|UpdateInventory))))

(fn PlaceObject
  (params (Index :type Integer))
  (bind _inventorycontent (Variables|Default|GetInventoryContent))
  (bind _output (Utilities|Array|Get(acopy) _inventorycontent))
  (LocalVariables|SetLOCAL_ItemID (.itemid _output))
  (LocalVariables|SetLOCAL_ItemQuantity (.quantity _output))
  (Utilities|FlowControl|Sequence
    (:then_0
      (CallFunction|RemovefromInventory Index false false))
    (:then_1
      (CallFunction|UpdateInventory))))

(fn PlaceItem(Helper)
  (params (ItemID :type Name))
  (Game|SpawnActorfromClass (.ItemClass (Utilities|Struct|BreakSTR_InventoryItem (Helper|GetItemData ItemID))) (Math|Transform|MakeTransform (Helper|GetPlacementLocation) "0, 0, 0" "1.000000,1.000000,1.000000") "AdjustIfPossibleButAlwaysSpawn" "MultiplyWithRoot" 0 0))

(fn QueryInventory
  (params (ItemID :type Name) (Quantity :type Integer))
  (for _array_element (Variables|Default|GetInventoryContent)
    (if (== (.ItemID (Utilities|Struct|BreakSTR_InventorySlot _array_element)) ItemID)
      (LocalVariables|SetTotalQuantity (+ (.Quantity (Utilities|Struct|BreakSTR_InventorySlot _array_element)) (LocalVariables|GetTotalQuantity)))))
  (return (>= (LocalVariables|GetTotalQuantity) Quantity) (LocalVariables|GetTotalQuantity)))