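; Base Blueprint for game machine items, tracking earnings, wear, repair and resale value.
; Using an unbroken machine adds test income, and every set number of uses reduces durability, scaled by the machine properties component, until it breaks.
; Repairing charges the player through the game mode and restores durability, but never clears the broken flag.
; Sell cost derives from the item data table value, scaled and clamped by durability, with a lower multiplier for broken machines.
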(fn ConstructionScript
  (|CallParentFunction))

(fn UpdateSellCost
  (bind _returnvalue (Utilities|GetDataTableRow "/Game/Inventory/DT_ItemData.DT_ItemData" (.RowName (Utilities|Struct|BreakDataTableRowHandle (Variables|/Game/Inventory/AC_ItemDataComponent.AC_ItemDataComponent_C|GetItemID (Variables|Default|GetAC_ItemDataComponent)))))
    (:then
      ;[0.6535 1 0] if the machine is broken, always just set to 0.2*value
      (if (Variables|Default|GetIsBroken?)
        (Variables|Default|SetCurrentSellCost (Math|Float|Floor (* (.ValueYen (Utilities|Struct|BreakSTR_InventoryItem _returnvalue)) (LocalVariables|GetBrokenMultiplier_LOCAL))))
        (else
          ;[0 1 0.2823] If the machine is fully repaired, always set to 0.8*value
          (if (>= (Variables|Default|GetDurabilityDecimal) 1.0)
            (Variables|Default|SetCurrentSellCost (Math|Float|Floor (* (.ValueYen (Utilities|Struct|BreakSTR_InventoryItem _returnvalue)) (LocalVariables|GetStandardMultiplier_High_LOCAL))))
            (else
              ;[0 1 0.9465] at any other state, multiply by 0.8 and the durability (ex: 0.75), and clamp between (value*0.4) and (value*0.8)
              (Variables|Default|SetCurrentSellCost (Math|Integer|Clamp(Integer) (Math|Float|Floor (* (.ValueYen (Utilities|Struct|BreakSTR_InventoryItem _returnvalue)) (LocalVariables|GetStandardMultiplier_High_LOCAL) (Variables|Default|GetDurabilityDecimal))) (Math|Float|Floor (* (.ValueYen (Utilities|Struct|BreakSTR_InventoryItem _returnvalue)) (LocalVariables|GetStandardMultiplier_Low_LOCAL))) (Math|Float|Floor (* (.ValueYen (Utilities|Struct|BreakSTR_InventoryItem _returnvalue)) (LocalVariables|GetStandardMultiplier_High_LOCAL))))))))))))

(fn UseMachine
  (if (not (Variables|Default|GetIsBroken?))
    ;[0 1 0.437] (TEST) add money to the machine, print out earned total for that machine
    (bind _output_get (Variables|Default|SetMoneyEarned (+ (Variables|Default|GetMoneyEarned) 100)))
    (Development|PrintString (Utilities|String|ToString(Integer) _output_get) true true "(R=1.000000,G=0.000000,B=0.127446,A=1.000000)")
    (bind _result (Math|Integer|IncrementInt (Variables|Default|GetUseCounter))
      (:%20%20
        (if (>= _result (Variables|/Game/Inventory/Items/Games_Machines/AC_MachineProperties.AC_MachineProperties_C|GetNumUsesToDamage (Variables|Default|GetAC_MachineProperties)))
          (CallFunction|DamageMachine)
          (Variables|Default|SetUseCounter 0))))))

(fn DamageMachine
  (Variables|Default|SetIsNew? false)
  (bind _output_get (Variables|Default|SetDurabilityDecimal (- (Variables|Default|GetDurabilityDecimal) (* (Variables|/Game/Inventory/Items/Games_Machines/AC_MachineProperties.AC_MachineProperties_C|GetDurabilityModifier (Variables|Default|GetAC_MachineProperties)) (LocalVariables|GetDefaultDamageAmount_LOCAL)))))
  (if (<= _output_get 0.0)
    (Variables|Default|SetIsBroken? true)))

(fn RepairMachine
  (bind _ac_machineproperties (Variables|Default|GetAC_MachineProperties))
  (bind _asbp_third_person_gamemode_als (Utilities|Casting|CastToBP_ThirdPersonGamemode_ALS (Game|GetGameMode)))
  (Default|AlterMoney _asbp_third_person_gamemode_als (* (Variables|/Game/Inventory/Items/Games_Machines/AC_MachineProperties.AC_MachineProperties_C|GetRepairCost _ac_machineproperties) -1))
  (bind _output_get (Variables|Default|SetDurabilityDecimal (Math|Float|Clamp(Float) (+ (Variables|Default|GetDurabilityDecimal) (Variables|/Game/Inventory/Items/Games_Machines/AC_MachineProperties.AC_MachineProperties_C|GetDurabilityRepairAmount _ac_machineproperties)))))
  (Development|PrintText (Utilities|Text|FormatText "machine: {x} has been repaired." (Utilities|GetObjectName self)) true true "(R=1.000000,G=0.354504,B=0.000000,A=1.000000)")
  (if (>= _output_get 1.0)
    (Variables|Default|SetIsNew? true)))